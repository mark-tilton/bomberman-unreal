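; Player character Blueprint with axis-driven movement and look, jumping, and bomb placement.
; The Throwbomb input passes an authority check before CreateBomb spawns a Bomb just in front of the actor, with no remote branch wired.
; On BeginPlay it binds Death to its OnDestroyed event, which spawns the game mode's spectator class at the world origin without possessing it.
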(event `InputAxis|MoveForward`
  (params (AxisValue :type "Float (single-precision)"))
  (`self.AddMovementInput` (`KismetMathLibrary.GetForwardVector` (`self.K2_GetActorRotation`)) AxisValue))

(event `InputAxis|LookVertical`
  (params (AxisValue :type "Float (single-precision)"))
  (`self.AddControllerPitchInput` AxisValue))

(event `InputAxis|LookHorizontal`
  (params (AxisValue :type "Float (single-precision)"))
  (`self.AddControllerYawInput` AxisValue))

(event `InputAxis|StrafeRight`
  (params (AxisValue :type "Float (single-precision)"))
  (`self.AddMovementInput` (`KismetMathLibrary.GetRightVector` (`self.K2_GetActorRotation`)) AxisValue))

(event `InputAction|Throwbomb`
  (:`Pressed`
    (`/Engine/EditorBlueprintResources/ActorMacros.Switch Has Authority`
      (:`Authority`
        (`self.CreateBomb`)))))

(event `CreateBomb`
  ;[1 1 1] Bomb Placed Event
  (`|SpawnActorFromClass` "/Game/Blueprints/Bomb.Bomb_C" (`KismetMathLibrary.Conv_VectorToTransform` (+ (* (`KismetMathLibrary.GetForwardVector` (`self.K2_GetActorRotation`)) 50.0) (`self.K2_GetActorLocation`)))))

(event `InputAction|Jump`
  (:`Pressed`
    (`self.Jump`)))

(event `self.ReceiveBeginPlay`
  (add `self.OnDestroyed` (delegate `Death`)))

(event `Death`
  (`|SpawnActorFromClass` (`GameMode.SpectatorClass` (`GameplayStatics.GetGameMode`)) (`KismetMathLibrary.MakeTransform` (0.0 0.0 0.0))))

(fn `UserConstructionScript`)