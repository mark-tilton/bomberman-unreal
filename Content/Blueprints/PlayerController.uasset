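; Player controller Blueprint that handles bomb throwing and a switch to spectating on death, with movement and look inputs left as empty stubs.
; The Throwbomb press spawns a Bomb at a fixed point near the world origin, since its forward vector and base location use zero defaults.
; BeginPlay binds OnDestroyed to Death, which spawns the game mode's spectator class at the origin without possessing it.
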(event `InputAxis|MoveForward`
  (params (AxisValue :type "Float (single-precision)")))

(event `InputAxis|LookVertical`
  (params (AxisValue :type "Float (single-precision)")))

(event `InputAxis|LookHorizontal`
  (params (AxisValue :type "Float (single-precision)")))

(event `InputAxis|StrafeRight`
  (params (AxisValue :type "Float (single-precision)")))

(event `InputAction|Throwbomb`
  (:`Pressed`
    (`|SpawnActorFromClass` "/Game/Blueprints/Bomb.Bomb_C" (`KismetMathLibrary.Conv_VectorToTransform` (+ (* (`KismetMathLibrary.GetForwardVector` (struct)) 50.0) (0.0 0.0 0.0))))))

(event `InputAction|Jump`)

(event `self.ReceiveBeginPlay`
  (add `self.OnDestroyed` (delegate `Death`)))

(event `Death`
  (`|SpawnActorFromClass` (`GameMode.SpectatorClass` (`GameplayStatics.GetGameMode`)) (`KismetMathLibrary.MakeTransform` (0.0 0.0 0.0))))

(fn `UserConstructionScript`)