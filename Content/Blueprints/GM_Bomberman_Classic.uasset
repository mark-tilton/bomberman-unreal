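; Bomberman classic level Blueprint that builds the arena's floor and outer walls in its construction script.
; A single loop over Width × Height converts each index to a 200-unit grid position, using a hardcoded row length of 15.
; Every cell gets a mossy floor mesh, and border cells get a raised wall mesh.
; Border cells in odd columns receive a second mesh at the same position.
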(fn `UserConstructionScript`
  ;[1 1 1] Itterate through indicies
  (for _index (range (* (`self.width`) (`self.height`)))
    (bind _returnvalue (mod _index 15))
    (bind _returnvalue_2 (`KismetMathLibrary.Conv_IntToDouble` (* _returnvalue 200)))
    (bind _returnvalue_3 (/ _index 15))
    (bind _returnvalue_4 (`KismetMathLibrary.Conv_IntToDouble` (* _returnvalue_3 200)))
    ;[1 1 1] Make floor
    (bind _returnvalue_5 (`AddComponent|StaticMeshComponent_8` :`bManualAttachment` true :`RelativeTransform` (`KismetMathLibrary.Conv_VectorToTransform` (`KismetMathLibrary.MakeVector` _returnvalue_2 _returnvalue_4))))
    (`PrimitiveComponent.SetMaterial` _returnvalue_5 0 "/Game/Materials/M_Ground_Moss.M_Ground_Moss")
    ;[1 1 1] Make outer walls
    (if (or (or (== _returnvalue 0) (== _returnvalue (- (`self.width`) 1))) (or (== _returnvalue_3 0) (== _returnvalue_3 (- (`self.height`) 1))))
      (bind _returnvalue_6 (`KismetMathLibrary.Conv_VectorToTransform` (`KismetMathLibrary.MakeVector` _returnvalue_2 _returnvalue_4 250.0)))
      (`AddComponent|StaticMeshComponent_5` :`RelativeTransform` _returnvalue_6)
      (if (!= (mod _returnvalue 2) 0)
        (`AddComponent|StaticMeshComponent_20094` :`RelativeTransform` _returnvalue_6)))))