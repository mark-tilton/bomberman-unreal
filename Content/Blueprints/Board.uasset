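; Grid board actor that builds a Bomberman-style arena of walls, floor and randomly placed boxes.
; The construction script forces odd dimensions, then adds border walls, pillars on even cells and a scaled floor.
; On BeginPlay, the authority spawns boxes on unoccupied tiles by fill chance, gated by IsProtectedTile, whose corner-exclusion expression appears unconnected.
; It records BoxTransforms, which remotes loop over to spawn their own boxes; both OnRep functions are empty.
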(event `self.ReceiveBeginPlay`
  (bind _width (`self.width`))
  (bind _boxtransforms (`self.boxTransforms`))
  (`/Engine/EditorBlueprintResources/ActorMacros.Switch Has Authority`
    (:`Authority`
      ;[1 1 1] Itterate through indicies
      (for _index (range (* (`self.width`) (`self.height`)))
        (bind _returnvalue (mod _index _width))
        (bind _returnvalue_2 (/ _index _width))
        ;[1 1 1] Make boxes
        (if (and (`self.IsProtectedTile` _returnvalue _returnvalue_2) (< (`KismetMathLibrary.RandomFloat`) (`self.fillPercentage`)))
          (bind _returnvalue_3 (`KismetMathLibrary.MakeVector` (`KismetMathLibrary.Conv_IntToDouble` (* _returnvalue 200)) (`KismetMathLibrary.Conv_IntToDouble` (* _returnvalue_2 200)) 95.0))
          (bind (_outactors _returnvalue_4) (`KismetSystemLibrary.SphereOverlapActors_NEW` _returnvalue_3 1.0 (`|MakeArray` "ObjectTypeQuery2" :!type "EngineTypes.EObjectTypeQuery Enum")))
          (if (not _returnvalue_4)
            (bind _returnvalue_5 (`|SpawnActorFromClass` "/Game/Blueprints/Box.Box_C" (`KismetMathLibrary.Conv_VectorToTransform` _returnvalue_3)))
            (`KismetArrayLibrary.Array_Add` (`self.boxTransforms`) (`self.GetTransform` _returnvalue_5))))))
    (:`Remote`
      (for _index_2 (range (+ (`KismetArrayLibrary.Array_Length` _boxtransforms) 1))
        (`|SpawnActorFromClass` "/Game/Blueprints/Box.Box_C" (`KismetArrayLibrary.Array_Get` _boxtransforms _index_2))))))

(fn `OnRep_boxes`)

(fn `OnRep_seed`)

(fn `UserConstructionScript`
  (bind _width (`self.width`))
  (bind _width_2 (`self.width`))
  (bind _height (`self.height`))
  (bind _returnvalue (`KismetMathLibrary.Conv_IntToDouble` (`self.width`)))
  (bind _returnvalue_2 (`KismetMathLibrary.Conv_IntToDouble` (`self.height`)))
  ;[1 1 1] Ensure width/height are odd
  (if (== (mod _width_2 2) 0)
    (set `self.width` (+ _width_2 1)))
  (if (== (mod _height 2) 0)
    (set `self.height` (+ _height 1)))
  ;[1 1 1] Itterate through indicies
  (for _index (range (* (`self.width`) (`self.height`)))
    (bind _returnvalue_3 (mod _index _width))
    (bind _returnvalue_4 (/ _index _width))
    ;[1 1 1] Make outer walls
    (if (or (== _returnvalue_3 0) (== _returnvalue_3 (- (`self.width`) 1)) (== _returnvalue_4 0) (== _returnvalue_4 (- (`self.height`) 1)))
      (bind _returnvalue_5 (`KismetMathLibrary.Conv_IntToDouble` (* _returnvalue_3 200)))
      (bind _returnvalue_6 (`KismetMathLibrary.Conv_IntToDouble` (* _returnvalue_4 200)))
      (bind _returnvalue_7 (`AddComponent|StaticMeshComponent_107147` :`RelativeTransform` (`KismetMathLibrary.Conv_VectorToTransform` (`KismetMathLibrary.MakeVector` _returnvalue_5 _returnvalue_6 250.0))))
      (`PrimitiveComponent.SetMaterial` _returnvalue_7 0 "/Game/StarterContent/Materials/M_CobbleStone_Rough.M_CobbleStone_Rough")
      (else
        ;[1 1 1] Inner walls
        (if (and (== (mod _returnvalue_3 2) 0) (== (mod _returnvalue_4 2) 0))
          (bind _returnvalue_8 (`AddComponent|StaticMeshComponent_107148` :`RelativeTransform` (`KismetMathLibrary.Conv_VectorToTransform` (`KismetMathLibrary.MakeVector` _returnvalue_5 _returnvalue_6 150.0))))
          (`PrimitiveComponent.SetMaterial` _returnvalue_8 0 "/Game/StarterContent/Materials/M_CobbleStone_Rough.M_CobbleStone_Rough")))))
  ;[1 1 1] Make floor
  (`AddComponent|StaticMeshComponent_20015` :`RelativeTransform` (`KismetMathLibrary.MakeTransform` (`KismetMathLibrary.MakeVector` (/ (* _returnvalue 200.0) 2.0) (/ (* _returnvalue_2 200.0) 2.0) -50.0) (struct) (`KismetMathLibrary.MakeVector` _returnvalue _returnvalue_2 10.0))))